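; Guard NPC AI controller that runs the GuardBehaviour tree on the GuardBlackBoard and feeds it perception results.
; Sight of an actor not tagged Guard stores it as EnemyLocation and signals a focus change; losing sight or unpossessing clears both.
; Other senses record the non-guard actor's current position as LastSeenLocation.
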(event `self.ReceiveBeginPlay`
  (bind _blackboardcomponent (`self.UseBlackboard` "/Game/Dynamic/NPC/AI_Blueprint/GuardBlackBoard.GuardBlackBoard"))
  (set `self.BlackBoardComponent` _blackboardcomponent)
  (`self.RunBehaviorTree` "/Game/Dynamic/NPC/AI_Blueprint/GuardBehaviour.GuardBehaviour")
  (cast `/Game/Dynamic/NPC/Character/TP_Character` (`self.K2_GetPawn`)))

(event `self.OnUnpossess`
  (params (UnpossessedPawn :type "Pawn Object Reference"))
  (`BlackboardComponent.ClearValue` (`self.BlackBoardComponent`) (`self.EnemyLocation`))
  (`self.AI_FocusChange` false))

(event `self.AIPerception.OnTargetPerceptionUpdated`
  (params (Actor :type "Actor Object Reference") (Stimulus :type "AIStimulus Structure"))
  (bind _returnvalue (`self.ActorHasTag` Actor "Guard"))
  (bind _returnvalue_2 (`AIPerceptionSystem.GetSenseClassForStimulus` Stimulus))
  (if (== _returnvalue_2 "/Script/AIModule.AISense_Sight")
    (if (not _returnvalue)
      (`self.ShouldBlackboardSetEnemyLocation` Actor Stimulus))
    (elif (not _returnvalue)
      (`BlackboardComponent.SetValueAsVector` (`self.BlackBoardComponent`) (`self.LastSeenLocation`) (`self.K2_GetActorLocation` Actor)))))

(fn `ShouldBlackboardSetEnemyLocation`
  (params (ObjectValue :type "Object Object Reference") (AIStimulus :type "AIStimulus Structure (by ref)"))
  (bind _enemylocation (`self.EnemyLocation`))
  (bind _blackboardcomponent (`self.BlackBoardComponent`))
  (if (`.bSuccessfullySensed` (break `AIStimulus` AIStimulus))
    (`BlackboardComponent.SetValueAsObject` _blackboardcomponent _enemylocation ObjectValue)
    (`self.AI_FocusChange` true)
    (else
      (`BlackboardComponent.ClearValue` _blackboardcomponent _enemylocation)
      (`self.AI_FocusChange` false))))

(fn `UserConstructionScript`)