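; Game mode that builds an endless terrain from chained BP_Tile actors.
; On BeginPlay it fills the bounds volume pool, then spawns the initial tiles, passing each the shared ActorPool.
; Each tile's attach location becomes the next spawn transform.
; DestroyFirstTileWhenGreater trims the oldest tile and its attached actors once the tile count exceeds a given maximum; nothing in this graph calls it.
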(event `self.ReceiveBeginPlay`
  (`self.PopulateBoundsVolumePool`)
  (for _ (range 2)
    (`self.SpawnTile`)))

(fn `DestroyFirstTileWhenGreater`
  (params (MaxTilesAmount :type Integer))
  (bind _tiles (`self.Tiles`))
  (bind _output (`|GetArrayItem` _tiles))
  (if (> (`KismetArrayLibrary.Array_Length` (`self.Tiles`)) MaxTilesAmount)
    (bind _children (`/DatasmithContent/Blueprints/FBXImporter/FBXImporterUtils.GetAllAttachedActors` _output))
    (for _array_element _children
      (`self.K2_DestroyActor` _array_element))
    (`self.K2_DestroyActor` _output)
    (`KismetArrayLibrary.Array_Remove` _tiles)))

(fn `SpawnTile`
  (bind _returnvalue (`|SpawnActorFromClass` "/Game/Dynamic/Terrain/BP_Tile.BP_Tile_C" (`self.NextTileTransform`) "AlwaysSpawn" "OverrideRootScale" null null))
  (`Tile.SetPoolReference` _returnvalue (`self.ActorPool`))
  (set `self.NextTileTransform` (`/Game/Dynamic/Terrain/BP_Tile.GetAttachLocation` _returnvalue))
  (`KismetArrayLibrary.Array_Add` (`self.Tiles`) _returnvalue))

(fn `UserConstructionScript`)