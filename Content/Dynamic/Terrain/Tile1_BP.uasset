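; Terrain tile for an endless level, with a barrier that gates the player's passage and an Arrow marking the attach transform and forward direction.
; The barrier starts locked (red, collidable) and turns passable green when the player enters UnlockTrigger.
; An actor leaving LockTrigger along the Arrow's forward, judged by velocity dot product, relocks it and has InfiniteTerrainGameMode spawn a tile and trim the oldest beyond three.
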(event `self.ReceiveBeginPlay`
  (`self.LockBarrier`))

(event `self.LockTrigger.OnComponentEndOverlap`
  (params (OverlappedComponent :type "PrimitiveComponent Object Reference") (OtherActor :type "Actor Object Reference") (OtherComp :type "PrimitiveComponent Object Reference") (OtherBodyIndex :type Integer))
  (bind _asinfinite_terrain_game_mode (cast `/Game/Dynamic/InfiniteTerrainGameMode` (`GameplayStatics.GetGameMode`) :!pure true))
  (if (`self.IsPlayerExiting` OtherActor)
    (`self.LockBarrier`)
    (`/Game/Dynamic/InfiniteTerrainGameMode.SpawnTile` _asinfinite_terrain_game_mode)
    (`/Game/Dynamic/InfiniteTerrainGameMode.DestroyFirstTileWhenGreater` _asinfinite_terrain_game_mode 3)))

(event `self.UnlockTrigger.OnComponentBeginOverlap`
  (params (OverlappedComponent :type "PrimitiveComponent Object Reference") (OtherActor :type "Actor Object Reference") (OtherComp :type "PrimitiveComponent Object Reference") (OtherBodyIndex :type Integer) (bFromSweep :type Boolean) (SweepResult :type "HitResult Structure (by ref)"))
  (if (== OtherActor (`GameplayStatics.GetPlayerCharacter` 0))
    (`self.UnlockBarrier`)))

(fn `GetAttachLocation`
  (returns (ReturnValue :type "Transform Structure"))
  (return (`SceneComponent.K2_GetComponentToWorld` (`self.Arrow`))))

(fn `IsPlayerExiting`
  (params (Actor :type "Actor Object Reference"))
  (returns (ReturnValue :type Boolean))
  (bind _returnvalue (`KismetMathLibrary.Dot_VectorVector` (`KismetMathLibrary.Normal` (`self.GetVelocity` Actor)) (`SceneComponent.GetForwardVector` (`self.Arrow`))))
  (return (or (`KismetMathLibrary.InRange_FloatFloat` _returnvalue 0.0 90.0) (`KismetMathLibrary.InRange_FloatFloat` _returnvalue 270.0 360.0))))

(fn `LockBarrier`
  (`PrimitiveComponent.SetCollisionEnabled` (`self.Barrier`) "QueryAndPhysics")
  (`PrimitiveComponent.SetMaterial` (`self.Barrier`) 0 "/Game/Dynamic/Terrain/BarrierMaterial_Red_Inst.BarrierMaterial_Red_Inst"))

(fn `UnlockBarrier`
  (bind _barrier (`self.Barrier`))
  (`PrimitiveComponent.SetCollisionEnabled` _barrier "NoCollision")
  (`PrimitiveComponent.SetMaterial` _barrier 0 "/Game/Dynamic/Terrain/BarrierMaterial_Green_Inst.BarrierMaterial_Green_Inst"))

(fn `UserConstructionScript`)