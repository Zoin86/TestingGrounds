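; BP_Tile is one segment of an infinite terrain, scattered with random containers, rocks, sandbags and crates on begin play.
; Its barrier starts locked (red, solid) and turns green and passable when the player enters the unlock trigger.
; Leaving the lock trigger along the arrow's forward direction relocks it and has the game mode spawn a tile, then cull the oldest beyond a limit.
; The arrow also supplies the tile's attach transform.
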(event OnComponentEndOverlap(LockTrigger)
  (params (OverlappedComponent :type Primitive%20Component%20Object%20Reference) (OtherActor :type Actor%20Object%20Reference) (OtherComp :type Primitive%20Component%20Object%20Reference) (OtherBodyIndex :type Integer))
  (bind _returnvalue (Game|GetGameMode))
  (bind _asinfinite_terrain_game_mode (Utilities|Casting|CastToInfiniteTerrainGameMode _returnvalue))
  (if (and (== (Game|GetPlayerCharacter (stale _index)) OtherActor) (CallFunction|IsPlayerExiting OtherActor))
    (CallFunction|LockBarrier)
    (Default|SpawnTile _asinfinite_terrain_game_mode)
    (Utilities|FlowControl|Delay 0.05)
    (Default|DestroyFirstTilewhenGreater _asinfinite_terrain_game_mode 3)))

(event OnComponentBeginOverlap(UnlockTrigger)
  (params (OverlappedComponent :type Primitive%20Component%20Object%20Reference) (OtherActor :type Actor%20Object%20Reference) (OtherComp :type Primitive%20Component%20Object%20Reference) (OtherBodyIndex :type Integer) (bFromSweep :type Boolean) (SweepResult :type Hit%20Result%20Structure%20%28by%20ref%29))
  (if (== OtherActor (Game|GetPlayerCharacter 0))
    (CallFunction|UnlockBarrier)))

(event EventBeginPlay
  (CallFunction|LockBarrier)
  (Class|Tile|PlaceActors "/Game/Dynamic/Terrain/Props/BP_ContainerOpen.BP_ContainerOpen_C" 1 3 0.0 0.0)
  (Class|Tile|PlaceActors "/Game/Dynamic/Terrain/Props/BP_Rock.BP_Rock_C" 0 5 0.0 359.0)
  (Class|Tile|PlaceActors "/Game/Dynamic/Terrain/Props/BP_Rock2.BP_Rock2_C" 0 5 0.0 359.0)
  (Class|Tile|PlaceActors "/Game/Dynamic/Terrain/Props/BP_Rock3.BP_Rock3_C" 0 5 0.0 359.0)
  (Class|Tile|PlaceActors "/Game/Dynamic/Terrain/Props/BP_SandBag.BP_SandBag_C" 1 3 0.0 0.0)
  (Class|Tile|PlaceActors "/Game/Dynamic/Terrain/Props/BP_Crate.BP_Crate_C" 3 7 0.0 0.0))

(fn ConstructionScript)

(fn GetAttachLocation
  (return (Transformation|GetWorldTransform (Variables|Default|GetArrow))))

(fn UnlockBarrier
  (bind _barrier (Variables|Default|GetBarrier))
  (Collision|SetCollisionEnabled _barrier "NoCollision")
  (Rendering|Material|SetMaterial _barrier 0 "/Game/Dynamic/Terrain/MI_Barrier_Green.MI_Barrier_Green"))

(fn LockBarrier
  (Collision|SetCollisionEnabled (Variables|Default|GetBarrier) "QueryAndPhysics")
  (Rendering|Material|SetMaterial (Variables|Default|GetBarrier) 0 "/Game/Dynamic/Terrain/MI_BarrierMaterial_Red.MI_BarrierMaterial_Red"))

(fn IsPlayerExiting
  (params (Actor :type Actor%20Object%20Reference))
  (bind _returnvalue (Transformation|GetVelocity Actor))
  (bind _arrow (Variables|Default|GetArrow))
  (bind _returnvalue_2 (Math|Vector|Normalize _returnvalue))
  (bind _returnvalue_3 (Math|Vector|GetForwardVector _arrow))
  (bind _returnvalue_4 (Math|Vector|DotProduct _returnvalue_2 _returnvalue_3))
  (return (or (Math|Float|InRange(Float) _returnvalue_4 0.0 9e+01) (Math|Float|InRange(Float) _returnvalue_4 2.7e+02 3.6e+02))))